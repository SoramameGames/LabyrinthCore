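; Player controller that turns mouse input into touch-style gestures on non-mobile platforms and shows the cursor on start.
; Left and right buttons act as two fingers, feeding per-finger state in InputData and a finger count.
; OnPress, OnMove and OnRelease use these to dispatch one- and two-finger press, swipe, release and tap events, averaging two-finger positions.
; Taps are judged by time and distance limits; the mouse wheel drives pinch zoom.
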(event `self.ReceiveBeginPlay`
  (`self.SetDefaultInputType`))

(event `InputTouch`
  (params (Location :type "Vector Structure") (FingerIndex :type "ETouchIndex Enum")))

(event `Key|LeftMouseButton`
  (params (Key :type "Key Structure"))
  (bind (_locationx _locationy) (`WidgetLayoutLibrary.GetMousePositionScaledByDPI` (`GameplayStatics.GetPlayerController` 0)))
  (bind (_locationx_2 _locationy_2) (`WidgetLayoutLibrary.GetMousePositionScaledByDPI` (`GameplayStatics.GetPlayerController` 0)))
  ;[1 1 1] マウス用インプットシステム
  (:`Pressed`
    (if (not (`/Game/LabyrinthCore/Blueprints/Core/BPFL_Labyrinth.IsRunningOnMobile`))
      (`self.InputPressed` (`KismetMathLibrary.MakeVector` _locationx _locationy 0.0))
      (`self.AddFingerNum`)
      (`self.OnPress` "Touch1")))
  (:`Released`
    (if (not (`/Game/LabyrinthCore/Blueprints/Core/BPFL_Labyrinth.IsRunningOnMobile`))
      (`self.InputReleased` (`KismetMathLibrary.MakeVector` _locationx_2 _locationy_2))
      (`self.OnRelease` "Touch1")
      (`self.SubFingerNum`))))

(event `Key|RightMouseButton`
  (params (Key :type "Key Structure"))
  (bind (_locationx _locationy) (`WidgetLayoutLibrary.GetMousePositionScaledByDPI` (`GameplayStatics.GetPlayerController` 0)))
  (bind (_locationx_2 _locationy_2) (`WidgetLayoutLibrary.GetMousePositionScaledByDPI` (`GameplayStatics.GetPlayerController` 0)))
  ;[1 1 1] マウス用インプットシステム
  (:`Pressed`
    (if (not (`/Game/LabyrinthCore/Blueprints/Core/BPFL_Labyrinth.IsRunningOnMobile`))
      (`self.InputPressed` (`KismetMathLibrary.MakeVector` _locationx _locationy) "Touch2")
      (`self.AddFingerNum`)
      (`self.OnPress` "Touch2")))
  (:`Released`
    (if (not (`/Game/LabyrinthCore/Blueprints/Core/BPFL_Labyrinth.IsRunningOnMobile`))
      (`self.InputReleased` (`KismetMathLibrary.MakeVector` _locationx_2 _locationy_2) "Touch2")
      (`self.OnRelease` "Touch2")
      (`self.SubFingerNum`))))

(event `InputAxis|MouseWheel`
  (params (AxisValue :type "Float (single-precision)"))
  (bind _returnvalue (+ (`self.Zoom`) (* AxisValue 150.0)))
  ;[1 1 1] マウス用インプットシステム
  (if (not (`/Game/LabyrinthCore/Blueprints/Core/BPFL_Labyrinth.IsRunningOnMobile`))
    (if (!= AxisValue 0.0)
      (set `self.ZoomDelta` (- (`self.Zoom`) _returnvalue))
      (set `self.Zoom` _returnvalue)
      (`self.Pinch`))))

(event `InputAxis|MouseX`
  (params (AxisValue :type "Float (single-precision)"))
  (bind (_locationx _locationy) (`WidgetLayoutLibrary.GetMousePositionScaledByDPI` (`GameplayStatics.GetPlayerController` 0)))
  ;[1 1 1] マウス用インプットシステム
  (if (not (`/Game/LabyrinthCore/Blueprints/Core/BPFL_Labyrinth.IsRunningOnMobile`))
    (if (!= AxisValue 0.0)
      (for (_array_element _array_index) (`self.InputData`) :!label _label
        (if (`|EnumInequality` (`.InputState_2_ED25E83C4EAAE7C4AE349192438E6B6A` (break `/Game/LabyrinthCore/Blueprints/Core/InputDataStruct` _array_element)) "NewEnumerator1")
          (bind _returnvalue (cast `ETouchIndex` (`KismetMathLibrary.Conv_IntToByte` _array_index)))
          (`self.InputMoved` (`KismetMathLibrary.MakeVector` _locationx _locationy) _returnvalue)))
      (`self.OnMove` _returnvalue))))

(event `InputAxis|MouseY`
  (params (AxisValue :type "Float (single-precision)"))
  ;[1 1 1] マウス用インプットシステム
  (if (not (`/Game/LabyrinthCore/Blueprints/Core/BPFL_Labyrinth.IsRunningOnMobile`))
    (if (!= AxisValue 0.0)
      (goto _label))))

(fn `AddFingerNum`
  (bind _sessionmaxfingernum (`self.SessionMaxFingerNum`))
  (`|ExecutionSequence`
    (:`then_0`
      (bind _result (`/Engine/EditorBlueprintResources/StandardMacros.IncrementInt` (`self.FingerNum`))
        (:`  `
          (set `self.SessionMaxFingerNum` (`KismetMathLibrary.SelectInt` _result _sessionmaxfingernum (> _result _sessionmaxfingernum))))))
    (:`then_1`
      (return))))

(fn `InputMoved`
  (params (Location :type "Vector Structure") (TouchIndex :type "ETouchIndex Enum" :default "Touch1"))
  (bind _returnvalue (`KismetMathLibrary.Conv_ByteToInt` TouchIndex))
  (bind _inputdata (`self.InputData`))
  (bind (_inputstate _touchlocation _touchdeltalocation _touchstartlocation _pressstarttime) (break `/Game/LabyrinthCore/Blueprints/Core/InputDataStruct` (`|GetArrayItem` _inputdata _returnvalue)))
  (if (`|EnumInequality` _inputstate "NewEnumerator1")
    (`KismetArrayLibrary.Array_Set` _inputdata _returnvalue (make `/Game/LabyrinthCore/Blueprints/Core/InputDataStruct` "NewEnumerator2" Location (- Location _touchlocation) _touchstartlocation _pressstarttime))))

(fn `InputPressed`
  (params (Location :type "Vector Structure") (TouchIndex :type "ETouchIndex Enum" :default "Touch1"))
  (`KismetArrayLibrary.Array_Set` (`self.InputData`) (`KismetMathLibrary.Conv_ByteToInt` TouchIndex) (make `/Game/LabyrinthCore/Blueprints/Core/InputDataStruct` "NewEnumerator0" Location (0.0 0.0 0.0) Location (`KismetMathLibrary.Now`))))

(fn `InputReleased`
  (params (Location :type "Vector Structure") (TouchIndex :type "ETouchIndex Enum" :default "Touch1"))
  (bind _returnvalue (`KismetMathLibrary.Conv_ByteToInt` TouchIndex))
  (bind _inputdata (`self.InputData`))
  (bind (_inputstate _touchlocation _touchdeltalocation _touchstartlocation _pressstarttime) (break `/Game/LabyrinthCore/Blueprints/Core/InputDataStruct` (`|GetArrayItem` _inputdata _returnvalue)))
  (`KismetArrayLibrary.Array_Set` _inputdata _returnvalue (make `/Game/LabyrinthCore/Blueprints/Core/InputDataStruct` "NewEnumerator1" _touchlocation _touchdeltalocation _touchstartlocation _pressstarttime)))

(fn `OnMove`
  (params (TouchIndex :type "ETouchIndex Enum" :default "Touch1"))
  (locals (InputTouchIndex :type "ETouchIndex Enum") (TouchLocationArray :type "Array of Vector Structure"))
  (bind _returnvalue (`KismetMathLibrary.GetVectorArrayAverage` (`local.TouchLocationArray`)))
  (bind (_inputstate _touchlocation _touchdeltalocation) (break `/Game/LabyrinthCore/Blueprints/Core/InputDataStruct` (`|GetArrayItem` (`self.InputData`) (`KismetMathLibrary.Conv_ByteToInt` (`local.InputTouchIndex`)))))
  (set `local.InputTouchIndex` TouchIndex)
  (switch `int` (`self.FingerNum`)
    (:`1`
      ;[1 1 1] 1本指
      (if (`|EnumInequality` _inputstate "NewEnumerator1")
        (set `self.TouchLocation` _touchlocation)
        (set `self.TouchDeltaLocation` _touchdeltalocation)
        (`self.Swipe` (`local.InputTouchIndex`))))
    (:`2`
      ;[1 1 1] 2本指
      (for _array_element (`self.InputData`)
        (bind (_inputstate_2 _touchlocation_2) (break `/Game/LabyrinthCore/Blueprints/Core/InputDataStruct` _array_element))
        (if (`|EnumInequality` _inputstate_2 "NewEnumerator1")
          (bind _returnvalue_2 (`KismetArrayLibrary.Array_Add` (`local.TouchLocationArray`) _touchlocation_2))
          (if (>= _returnvalue_2 1)
            (break))))
      (set `self.TwoFingerTouchDeltaLocation` (- _returnvalue (`self.TwoFingerTouchLocation`)))
      (set `self.TwoFingerTouchLocation` _returnvalue)
      (`self.TwoFingerSwipe`))))

(fn `OnPress`
  (params (TouchIndex :type "ETouchIndex Enum" :default "Touch1"))
  (locals (InputTouchIndex :type "ETouchIndex Enum" :default "Touch1") (TouchLocationArray :type "Array of Vector Structure"))
  (set `local.InputTouchIndex` TouchIndex)
  (switch `int` (`self.FingerNum`)
    (:`1`
      ;[1 1 1] 1本指
      (set `self.TouchLocation` (`.TouchLocation_5_855BCCC64584017692B3E789170A3CBC` (break `/Game/LabyrinthCore/Blueprints/Core/InputDataStruct` (`|GetArrayItem` (`self.InputData`) (`KismetMathLibrary.Conv_ByteToInt` (`local.InputTouchIndex`))))))
      (set `self.TouchDeltaLocation` (0.0 0.0 0.0)) ; 移動量は 0 で初期化しておく
      (`self.Pressed` (`local.InputTouchIndex`)))
    (:`2`
      ;[1 1 1] 2本指
      (for _array_element (`self.InputData`)
        (bind (_inputstate _touchlocation) (break `/Game/LabyrinthCore/Blueprints/Core/InputDataStruct` _array_element))
        (if (`|EnumInequality` _inputstate "NewEnumerator1")
          (bind _returnvalue (`KismetArrayLibrary.Array_Add` (`local.TouchLocationArray`) _touchlocation))
          (if (>= _returnvalue 1)
            (break))))
      (set `self.TwoFingerTouchLocation` (`KismetMathLibrary.GetVectorArrayAverage` (`local.TouchLocationArray`)))
      (set `self.TwoFingerTouchDeltaLocation` (0.0 0.0 0.0)) ; 移動量は 0 で初期化しておく
      (`self.TwoFingerPressed`))))

(fn `OnRelease`
  (params (TouchIndex :type "ETouchIndex Enum" :default "Touch1"))
  (locals (TapLocationArray :type "Array of Vector Structure"))
  (bind _taplocationarray (`local.TapLocationArray`))
  (`|ExecutionSequence`
    (:`then_0`
      (switch `int` (`self.FingerNum`)
        (:`1`
          (`self.Released`))
        (:`2`
          (`self.TwoFingerReleased`))))
    (:`then_1`
      (for _array_element (`self.InputData`)
        (bind (_inputstate _touchlocation _touchdeltalocation _touchstartlocation _pressstarttime) (break `/Game/LabyrinthCore/Blueprints/Core/InputDataStruct` _array_element))
        ;[1 1 1] タップ入力が成功した指をADDする
        (if (and (< (`KismetMathLibrary.GetTotalSeconds` (- (`KismetMathLibrary.Now`) _pressstarttime)) (`self.TapJudgeLimitTime`)) (< (`KismetMathLibrary.VSize2D` (- (`KismetMathLibrary.Conv_VectorToVector2D` _touchlocation) (`KismetMathLibrary.Conv_VectorToVector2D` _touchstartlocation))) (`self.TapJudgeLimitLength`)))
          (`KismetArrayLibrary.Array_Add` (`local.TapLocationArray`) _touchlocation)))
      (switch `int` (`KismetArrayLibrary.Array_Length` _taplocationarray) ; ADDした本数によって種類を分ける
        (:`1`
          ;[1 1 1] 1本指タップ
          (set `self.TapLocation` (`|GetArrayItem` _taplocationarray))
          (`self.Tap`))
        (:`2`
          ;[1 1 1] 2本指タップ
          (set `self.TwoFingerTapLocation` (`KismetMathLibrary.GetVectorArrayAverage` (`local.TapLocationArray`)))
          (`self.TwoFingerTap`))))))

(fn `SetDefaultInputType`
  (`self.SetVirtualJoystickVisibility` false)
  (`/Game/LabyrinthCore/Blueprints/Core/BPFL_Labyrinth.ShowMouseCursor` true))

(fn `SubFingerNum`
  (bind _result (`/Engine/EditorBlueprintResources/StandardMacros.DecrementInt` (`self.FingerNum`))
    (:`  `
      (if (<= _result 0)
        (set `self.SessionMaxFingerNum` 0)))))

(fn `UserConstructionScript`)