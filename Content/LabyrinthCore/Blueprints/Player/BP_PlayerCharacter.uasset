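; Player character Blueprint for LabyrinthCore that provides a swipe-driven orbit camera, an outline mesh following the main mesh's pose, and an audio listener attached to the character.
; Swipes bound from the player controller add frame-time-scaled, clamped velocity to the camera when movement is allowed; the tap handler is empty.
; Each Tick applies that velocity to wrapped yaw and clamped pitch, repositions the spring arm in world space, then decays the velocity for inertia.
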(event `self.ReceiveBeginPlay`
  (bind _controller (`/Game/LabyrinthCore/Blueprints/Core/BPFL_Labyrinth.GetPlayerControllerBP`))
  (`parent.ReceiveBeginPlay`)
  (`|ExecutionSequence`
    (:`then_0`
      (`self.InitCameraControll`)
      (`PlayerController.SetAudioListenerOverride` :`self` (`GameplayStatics.GetPlayerController` 0) :`AttachToComponent` (`self.Mesh`)) ; サウンドリスナーの位置をカメラではなくキャラクターの位置になるように変更
    )
    (:`then_1`
      (add `/Game/LabyrinthCore/Blueprints/Player/BP_PlayerController.Tap` _controller (delegate `EventTap`))
      (add `/Game/LabyrinthCore/Blueprints/Player/BP_PlayerController.Swipe` _controller (delegate `EventSwipe`)))))

(event `EventSwipe`
  (params (TouchIndex :type "ETouchIndex Enum" :default "Touch1"))
  (`self.InputCameraControll`))

(event `EventTap`)

(event `self.ReceiveTick`
  (params (DeltaSeconds :type "Float (single-precision)"))
  (`parent.ReceiveTick` DeltaSeconds)
  (`self.UpdateCameraControll`))

(fn `InitCameraControll`
  ;[1 1 1] 初期パラメータの設定
  (set `self.CameraArmInitialRotation` (`self.K2_GetActorRotation`))
  (set `self.CameraArmInitialLocation` (`SceneComponent.RelativeLocation` (`self.SpringArm`)))
  (set `self.CameraArmLengthBefore` (`SpringArmComponent.TargetArmLength` (`self.SpringArm`)))
  (set `self.CameraFOV` (`CameraComponent.FieldOfView` (`self.Camera`))))

(fn `InputCameraControll`
  (bind (_touchdeltalocation_x _touchdeltalocation_y) (`KismetMathLibrary.BreakVector` (`/Game/LabyrinthCore/Blueprints/Player/BP_PlayerController.TouchDeltaLocation` (`/Game/LabyrinthCore/Blueprints/Core/BPFL_Labyrinth.GetPlayerControllerBP`))))
  (bind _returnvalue (/ 1.0 (* (`GameplayStatics.GetWorldDeltaSeconds`) 1000.0)))
  (if (and (`self.bCanMovePlayerCamera`) true)
    (`|ExecutionSequence`
      (:`then_0`
        ;[1 1 1] 加速度の計算
        (`|ExecutionSequence`
          (:`then_0`
            (set `self.CameraAccelX` (* _touchdeltalocation_x (`self.CameraAccelSpeedX`) _returnvalue)))
          (:`then_1`
            (set `self.CameraAccelY` (* _touchdeltalocation_y (`self.CameraAccelSpeedY`) _returnvalue -1.0)))))
      (:`then_1`
        ;[1 1 1] 算出した加速度をカメラ速度に反映
        (`|ExecutionSequence`
          (:`then_0`
            (set `self.CameraSpeedX` (`KismetMathLibrary.FClamp` (+ (`self.CameraSpeedX`) (`self.CameraAccelX`)) (* (`self.CameraMaxSpeedX`) -1.0) (`self.CameraMaxSpeedX`))))
          (:`then_1`
            (set `self.CameraSpeedY` (`KismetMathLibrary.FClamp` (+ (`self.CameraSpeedY`) (`self.CameraAccelY`)) (* (`self.CameraMaxSpeedY`) -1.0) (`self.CameraMaxSpeedY`)))))))))

(fn `UpdateCameraControll`
  (bind _springarm (`self.SpringArm`))
  (bind (_cameraarminitialrotation_roll _cameraarminitialrotation_pitch _cameraarminitialrotation_yaw) (`KismetMathLibrary.BreakRotator` (`self.CameraArmInitialRotation`)))
  (`|ExecutionSequence`
    (:`then_0`
      ;[1 1 1] カメラ回転値を更新
      (set `self.CameraRotateX` (mod (+ (`self.CameraRotateX`) (`self.CameraSpeedX`)) 360.0))
      (set `self.CameraRotateY` (`KismetMathLibrary.FClamp` (+ (`self.CameraRotateY`) (`self.CameraSpeedY`)) (`self.CameraRotateYMin`) (`self.CameraRotateYMax`))))
    (:`then_1`
      ;[1 1 1] カメラを更新
      (`SceneComponent.K2_SetWorldLocation` _springarm (+ (`self.K2_GetActorLocation`) (`self.CameraArmInitialLocation`)) false false) ; LookAtの位置を初期位置に戻してから計算を始める
      (`SceneComponent.K2_SetWorldRotation` _springarm (`KismetMathLibrary.MakeRotator` 0.0 (+ _cameraarminitialrotation_pitch (`self.CameraRotateY`)) (+ _cameraarminitialrotation_yaw (`self.CameraRotateX`))) false false))
    (:`then_2`
      ;[1 1 1] 速度を減衰させる
      (set `self.CameraSpeedX` (* (`self.CameraSpeedX`) (`self.CameraDecayX`)))
      (set `self.CameraSpeedY` (* (`self.CameraSpeedY`) (`self.CameraDecayY`))))))

(fn `UserConstructionScript`
  (`SkinnedMeshComponent.SetLeaderPoseComponent` (`self.OutlineMesh`) (`self.Mesh`) false) ; Meshのポーズをコピーするように設定
)