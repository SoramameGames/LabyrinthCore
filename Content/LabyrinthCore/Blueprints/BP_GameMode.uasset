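; Game mode for LabyrinthCore that sets up the player view, debug UI and frame cap.
; On BeginPlay it points player 0's camera at PlayerCharacter, adds WB_DebugUI in non-distribution builds, and caps the frame rate through a t.MaxFPS console command.
; SetFrameRate stores a new rate and builds the same command from it, but appends the number without a separating space.
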(event `self.ReceiveBeginPlay`
  (`|ExecutionSequence`
    (:`then_0`
      ;[1 1 1] プレイヤーカメラを設定
      (`PlayerController.SetViewTargetWithBlend` (`GameplayStatics.GetPlayerController` 0) (`self.PlayerCharacter`) 0.0 "VTBlend_Linear" 0.0 false))
    (:`then_1`
      ;[1 1 1] Debug用UMG追加
      (if (not (`KismetSystemLibrary.IsPackagedForDistribution`))
        (bind _returnvalue (`|CreateWidget` "/Game/LabyrinthCore/Blueprints/Debug/WB_DebugUI.WB_DebugUI_C"))
        (`UserWidget.AddToViewport` _returnvalue 0)))
    (:`then_2`
      (`KismetSystemLibrary.ExecuteConsoleCommand` "t.MaxFPS  30" null))))

(fn `SetFrameRate`
  (params (FrameRate :type Integer))
  (bind _output_get (set `self.FrameRate` FrameRate))
  (`KismetSystemLibrary.ExecuteConsoleCommand` (`KismetStringLibrary.Concat_StrStr` "t.MaxFPS " (`KismetStringLibrary.Conv_IntToString` _output_get)) null))

(fn `UserConstructionScript`)