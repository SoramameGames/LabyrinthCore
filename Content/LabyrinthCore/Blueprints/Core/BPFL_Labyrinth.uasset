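; Blueprint function library for the Labyrinth game, providing shared accessors and small platform and cursor helpers.
; Getters return the game mode, player controller 0 and game instance cast to their project Blueprint classes.
; IsRunningOnMobile switches on platform name but returns false on every branch, including iOS and Android, alongside the name.
; ShowMouseCursor sets cursor visibility through the controller getter, always showing it when IsInEditor is true.
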(fn `GetGameInstanceBP`
  (returns (MyGameInstance :type "/Game/LabyrinthCore/Blueprints/Core/BP_GameInstance Object Reference"))
  (bind _asbp_game_instance (cast `/Game/LabyrinthCore/Blueprints/Core/BP_GameInstance` (`GameplayStatics.GetGameInstance` null)))
  (return _asbp_game_instance))

(fn `GetGameModeBP`
  (returns (MyGame :type "/Game/LabyrinthCore/Blueprints/Core/BP_GameMode Object Reference"))
  (bind _asbp_game_mode (cast `/Game/LabyrinthCore/Blueprints/Core/BP_GameMode` (`GameplayStatics.GetGameMode` null)))
  (return _asbp_game_mode))

(fn `GetPlayerControllerBP`
  (returns (Controller :type "/Game/LabyrinthCore/Blueprints/Player/BP_PlayerController Object Reference"))
  (bind _asbp_player_controller (cast `/Game/LabyrinthCore/Blueprints/Player/BP_PlayerController` (`GameplayStatics.GetPlayerController` null)))
  (return _asbp_player_controller))

(fn `IsRunningOnMobile`
  (returns (bIsMobile :type Boolean) (PlatformName :type String))
  (bind _returnvalue (`GameplayStatics.GetPlatformName`))
  (switch `string` _returnvalue
    (:`Default`
      (return false _returnvalue))
    (:`IOS`
      _)
    (:`Android`
      _))
  (return false _returnvalue))

(fn `ShowMouseCursor`
  (params (bEnable :type Boolean))
  (set `PlayerController.bShowMouseCursor` (or bEnable (`LabyrinthBlueprintLibrary.IsInEditor`)) (`self.GetPlayerControllerBP` null)))