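; Touch-driven player character that walks to tapped points and carries an orbit camera.
; Taps from the player controller trace from screen into the world and feed hit points to AI MoveTo.
; Swipe, pinch (or PC wheel) and two-finger swipe add clamped speeds that Tick applies with decay to orbit, FOV zoom and pan, the latter two easing back on release.
; An outline mesh copies the body pose, and audio listens from the character.
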(event Custom|MoveToTarget
  (params (TargetLocation :type Vector))
  (AI|AIMoveTo self TargetLocation 0 5.0 false))

(event Custom|TapRaycast
  (bind _controller (CallFunction|GetPlayerControllerBP))
  (bind _returnvalue (Class|WidgetLayoutLibrary|GetViewportScale))
  (bind _taplocation (Variables|/Game/LabyrinthCore/Blueprints/BP_PlayerController.BP_PlayerController_C|GetTapLocation _controller))
  (bind _returnvalue_2 (* _taplocation _returnvalue))
  (bind (_x _y) (Math|Vector|BreakVector _returnvalue_2))
  (bind (_worldlocation _worlddirection) (Class|PlayerController|DeprojectScreenPositiontoWorld _controller _x _y))
  ;[1 1 1] レイキャストを飛ばす
  (bind _outhits (Collision|MultiLineTraceByChannel _worldlocation (+ _worldlocation (* _worlddirection (Variables|Move|GetRaycastMaxDistance))) "TraceTypeQuery1" false 0 "ForDuration"))
  (bind _array_element (Utilities|Array|ForEachLoopwithBreak _outhits)
    (:LoopBody
      (CallFunction|MovetoTarget (.ImpactPoint (Collision|BreakHitResult _array_element))))))

(event EventBeginPlay
  ;[1 0 0] Begin
  (|CallParentFunction)
  (|BeginPlay))

(event EventTick
  (params (DeltaSeconds :type Float%20%28single-precision%29))
  ;[1 0 0] Tick
  (|CallParentFunction DeltaSeconds)
  (|Tick))

(fn ConstructionScript
  (Class|SkinnedMeshComponent|SetMasterPoseComponent (Variables|Default|GetOutlineMesh) (Variables|Character|GetMesh) false) ; Meshのポーズをコピーするように設定
)

(fn InitCameraControll
  ;[1 1 1] 初期パラメータの設定
  (Variables|CameraMove|SetCameraArmInitialRotation (Transformation|GetActorRotation))
  (Variables|CameraMove|SetCameraArmInitialLocation (Variables|/Script/Engine.SceneComponent|GetRelativeLocation (Variables|Default|GetSpringArm)))
  (Variables|CameraZoom|SetCameraFOV (Variables|/Script/Engine.CameraComponent|GetFieldOfView (Variables|Default|GetCamera))))

(fn InputCameraMove
  (bind _controller (CallFunction|GetPlayerControllerBP))
  (bind _touchdeltalocation (Variables|/Game/LabyrinthCore/Blueprints/BP_PlayerController.BP_PlayerController_C|GetTouchDeltaLocation _controller))
  (if (Variables|Default|GetbCanMovePlayerCamera)
    (Utilities|FlowControl|Sequence
      (:then_0
        ;[1 1 1] 加速度の計算
        (Variables|CameraMove|SetCameraMoveAccelX (* (CallFunction|ApplyValueatFPS (.x _touchdeltalocation)) (Variables|CameraMove|GetCameraMoveAccelXRatio) 0.01))
        (Variables|CameraMove|SetCameraMoveAccelY (* (CallFunction|ApplyValueatFPS (.y _touchdeltalocation)) (Variables|CameraMove|GetCameraMoveAccelYRatio) 0.01)))
      (:then_1
        ;[1 1 1] 算出した加速度をカメラ速度に反映
        (Variables|CameraMove|SetCameraMoveSpeedX (Math|Float|Clamp(Float) (+ (Variables|CameraMove|GetCameraMoveSpeedX) (Variables|CameraMove|GetCameraMoveAccelX)) (* (Variables|CameraMove|GetCameraMoveMaxSpeedX) -1.0) (Variables|CameraMove|GetCameraMoveMaxSpeedX)))
        (Variables|CameraMove|SetCameraMoveSpeedY (Math|Float|Clamp(Float) (+ (Variables|CameraMove|GetCameraMoveSpeedY) (Variables|CameraMove|GetCameraMoveAccelY)) (* (Variables|CameraMove|GetCameraMoveMaxSpeedY) -1.0) (Variables|CameraMove|GetCameraMoveMaxSpeedY)))))))

(fn InputCameraZoom
  (bind _controller (CallFunction|GetPlayerControllerBP))
  (if (Variables|Default|GetbCanMovePlayerCamera)
    (if (.bIsMobile (CallFunction|IsRunningonMobile)) ; True : モバイル実機
      (if (< (Variables|/Game/LabyrinthCore/Blueprints/BP_PlayerController.BP_PlayerController_C|GetTwoFingerDeltaDot _controller) 0.0)
        (Utilities|FlowControl|Sequence :!label _label
          (:then_0
            ;[1 1 1] 加速度の計算
            (Variables|CameraZoom|SetCameraZoomAccel (* (CallFunction|ApplyValueatFPS (Variables|/Game/LabyrinthCore/Blueprints/BP_PlayerController.BP_PlayerController_C|GetTwoFingerDeltaLength (CallFunction|GetPlayerControllerBP))) (Variables|CameraZoom|GetCameraZoomAccelRatio) -0.01)))
          (:then_1
            ;[1 1 1] 算出した加速度をズーム速度に反映
            (Variables|CameraZoom|SetCameraZoomSpeed (Math|Float|Clamp(Float) (+ (Variables|CameraZoom|GetCameraZoomSpeed) (Variables|CameraZoom|GetCameraZoomAccel)) (* (Variables|CameraZoom|GetCameraZoomMaxSpeed) -1.0) (Variables|CameraZoom|GetCameraZoomMaxSpeed))))))
      (else
        ;[1 1 1] PCのときはマウスホイール操作なので指数０なら可
        (if (== (Variables|/Game/LabyrinthCore/Blueprints/BP_PlayerController.BP_PlayerController_C|GetFingerNum _controller) 0)
          (goto _label))))))

(fn InputCameraRotation
  (bind _controller (CallFunction|GetPlayerControllerBP))
  (bind _camerarotatespeedymax (Variables|CameraRotate|GetCameraRotateSpeedYMax))
  (bind _camerarotatespeedxmax (Variables|CameraRotate|GetCameraRotateSpeedXMax))
  (bind _twofingertouchdeltalocation (Variables|/Game/LabyrinthCore/Blueprints/BP_PlayerController.BP_PlayerController_C|GetTwoFingerTouchDeltaLocation _controller))
  (if (Variables|Default|GetbCanMovePlayerCamera)
    (if (>= (Variables|/Game/LabyrinthCore/Blueprints/BP_PlayerController.BP_PlayerController_C|GetTwoFingerDeltaDot (CallFunction|GetPlayerControllerBP)) 0.0)
      (Utilities|FlowControl|Sequence
        (:then_0
          ;[1 1 1] 加速度の計算
          (Variables|CameraRotate|SetCameraRotateAccelX (* (CallFunction|ApplyValueatFPS (.x _twofingertouchdeltalocation)) (Variables|CameraRotate|GetCameraRotateAccelRatio) 0.01))
          (Variables|CameraRotate|SetCameraRotateAccelY (* (CallFunction|ApplyValueatFPS (.y _twofingertouchdeltalocation)) (Variables|CameraRotate|GetCameraRotateAccelRatio) 0.01)))
        (:then_1
          ;[1 1 1] 算出した加速度をカメラ回転速度に反映
          (Variables|CameraRotate|SetCameraRotateSpeedX (Math|Float|Clamp(Float) (+ (Variables|CameraRotate|GetCameraRotateSpeedX) (Variables|CameraRotate|GetCameraRotateAccelX)) (* _camerarotatespeedxmax -1.0) _camerarotatespeedxmax))
          (Variables|CameraRotate|SetCameraRotateSpeedY (Math|Float|Clamp(Float) (+ (Variables|CameraRotate|GetCameraRotateSpeedY) (Variables|CameraRotate|GetCameraRotateAccelY)) (* _camerarotatespeedymax -1.0) _camerarotatespeedymax)))))))

(fn UpdateCameraMove
  (bind _springarm (Variables|Default|GetSpringArm))
  (bind _cameraarminitialrotation (Variables|CameraMove|GetCameraArmInitialRotation))
  (Utilities|FlowControl|Sequence
    (:then_0
      ;[1 1 1] カメラ移動値を更新
      (Variables|CameraMove|SetCameraMoveX (|(((x+540)%360)-180) (+ (Variables|CameraMove|GetCameraMoveX) (CallFunction|ApplyValueatFPS (Variables|CameraMove|GetCameraMoveSpeedX)))))
      (Variables|CameraMove|SetCameraMoveY (Math|Float|Clamp(Float) (+ (Variables|CameraMove|GetCameraMoveY) (CallFunction|ApplyValueatFPS (Variables|CameraMove|GetCameraMoveSpeedY))) (Variables|CameraMove|GetCameraMoveYMin) (Variables|CameraMove|GetCameraMoveYMax))))
    (:then_1
      ;[1 1 1] カメラ位置を更新
      (Transformation|SetWorldLocation _springarm (+ (Transformation|GetActorLocation) (Variables|CameraMove|GetCameraArmInitialLocation)) false false) ; LookAtの位置を初期位置に戻してから計算を始める
      (Transformation|SetWorldRotation _springarm (Math|Rotator|MakeRotator 0.0 (+ (.pitch _cameraarminitialrotation) (* (Variables|CameraMove|GetCameraMoveY) -1.0)) (+ (.yaw _cameraarminitialrotation) (Variables|CameraMove|GetCameraMoveX))) false false))
    (:then_2
      ;[1 1 1] 速度を減衰させる
      (Variables|CameraMove|SetCameraMoveSpeedX (- (Variables|CameraMove|GetCameraMoveSpeedX) (CallFunction|ApplyValueatFPS (- (Variables|CameraMove|GetCameraMoveSpeedX) (* (Variables|CameraMove|GetCameraMoveSpeedX) (Variables|CameraMove|GetCameraMoveDecayX))))))
      (Variables|CameraMove|SetCameraMoveSpeedY (- (Variables|CameraMove|GetCameraMoveSpeedY) (CallFunction|ApplyValueatFPS (- (Variables|CameraMove|GetCameraMoveSpeedY) (* (Variables|CameraMove|GetCameraMoveSpeedY) (Variables|CameraMove|GetCameraMoveDecayY)))))))))

(fn UpdateCameraZoom
  (Utilities|FlowControl|Sequence
    (:then_0
      ;[1 1 1] ズーム値を更新
      (Variables|CameraZoom|SetCameraZoom (Math|Float|Clamp(Float) (+ (Variables|CameraZoom|GetCameraZoom) (Variables|CameraZoom|GetCameraZoomSpeed)) (Variables|CameraZoom|GetCameraZoomMin) (Variables|CameraZoom|GetCameraZoomMax))))
    (:then_1
      ;[1 1 1] ズーム反映
      (Camera|SetFieldOfView (Variables|BP_PlayerCharacter_C|GetCamera (CallFunction|GetPlayerCharacterBP)) (+ (Variables|CameraZoom|GetCameraFOV) (* (Variables|CameraZoom|GetCameraZoom) -1.0))))
    (:then_2
      ;[1 1 1] ズーム速度を減衰させる
      (Variables|CameraZoom|SetCameraZoomSpeed (* (Variables|CameraZoom|GetCameraZoomSpeed) (Variables|CameraZoom|GetCameraZoomSpeedDecay)))
      ;[1 1 1] 指を離すとズームを戻す
      (if (!= (Variables|/Game/LabyrinthCore/Blueprints/BP_PlayerController.BP_PlayerController_C|GetFingerNum (CallFunction|GetPlayerControllerBP)) 2)
        (Variables|CameraZoom|SetCameraZoom (* (Variables|CameraZoom|GetCameraZoom) (Variables|CameraZoom|GetCameraZoomDecay)))))))

(fn UpdateCameraRotation
  (bind _camerarotatedecay (Variables|CameraRotate|GetCameraRotateDecay))
  (bind _camerarotatespeeddecay (Variables|CameraRotate|GetCameraRotateSpeedDecay))
  (Utilities|FlowControl|Sequence
    (:then_0
      ;[1 1 1] Pan値を算出
      (Variables|CameraRotate|SetCameraRotateX (Math|Float|Clamp(Float) (+ (Variables|CameraRotate|GetCameraRotateX) (Variables|CameraRotate|GetCameraRotateSpeedX)) (Variables|CameraRotate|GetCameraRotateXMin) (Variables|CameraRotate|GetCameraRotateXMax)))
      (Variables|CameraRotate|SetCameraRotateY (Math|Float|Clamp(Float) (+ (Variables|CameraRotate|GetCameraRotateY) (Variables|CameraRotate|GetCameraRotateSpeedY)) (Variables|CameraRotate|GetCameraRotateYMin) (Variables|CameraRotate|GetCameraRotateYMax))))
    (:then_1
      ;[1 1 1] カメラ回転を反映
      (Transformation|SetRelativeRotation (Variables|Default|GetCamera) (Math|Rotator|MakeRotator 0.0 (* (Variables|CameraRotate|GetCameraRotateY) -1.0) (* (Variables|CameraRotate|GetCameraRotateX) 1.0)) false false))
    (:then_2
      ;[1 1 1] 回転速度を減衰させる
      (Variables|CameraRotate|SetCameraRotateSpeedX (* (Variables|CameraRotate|GetCameraRotateSpeedX) _camerarotatespeeddecay))
      (Variables|CameraRotate|SetCameraRotateSpeedY (* (Variables|CameraRotate|GetCameraRotateSpeedY) _camerarotatespeeddecay))
      ;[1 1 1] 指を離すと回転を戻す
      (if (!= (Variables|/Game/LabyrinthCore/Blueprints/BP_PlayerController.BP_PlayerController_C|GetFingerNum (CallFunction|GetPlayerControllerBP)) 2)
        (Variables|CameraRotate|SetCameraRotateX (* (Variables|CameraRotate|GetCameraRotateX) _camerarotatedecay))
        (Variables|CameraRotate|SetCameraRotateY (* (Variables|CameraRotate|GetCameraRotateY) _camerarotatedecay))))))

(event Custom|EventTap
  ;[1 1 1] イベントを登録
  (CallFunction|TapRaycast))

(event Custom|EventSwipe
  (params (TouchIndex :type ETouchIndex%20Enum :default "Touch1"))
  ;[1 1 1] イベントを登録
  (Camera|InputCameraMove))

(event Custom|EventPinch
  ;[1 1 1] イベントを登録
  (Camera|InputCameraZoom))

(event Custom|EventTwoFingerSwipe
  ;[1 1 1] イベントを登録
  (Camera|InputCameraRotation))